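; Player controller that routes shared inputs to either the UI or the player character, depending on menu map and pause state.
; BeginPlay shows the main menu on the menu map, or otherwise creates a pause widget for the Pause action to toggle.
; In menus, axes, Validate and Back send messages to the active widget; in gameplay, they drive movement and jump, with Back unused.
; Cursor visibility follows the game instance's MouseMode.
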(event `self.ReceiveBeginPlay`
  (bind _returnvalue (`GameplayStatics.GetPlayerController` 0))
  ;[0 1 0] Event BeginPlay
  (bind _asbp_game_instance (cast `/Game/02_Blueprints/BP_GameInstance` (`GameplayStatics.GetGameInstance`)))
  (set `self.BP_GameInstance` _asbp_game_instance)
  (bind _asbp_player_character (cast `/Game/02_Blueprints/Character/BP_PlayerCharacter` (`GameplayStatics.GetPlayerCharacter` 0)))
  (set `self.BP_PlayerCharacter` _asbp_player_character)
  (if (`/Game/02_Blueprints/BP_GameInstance.OnMenuMap` (`self.BP_GameInstance`))
    (`WidgetBlueprintLibrary.SetInputMode_GameAndUIEx` _returnvalue)
    (set `PlayerController.bShowMouseCursor` (`/Game/02_Blueprints/BP_GameInstance.MouseMode` (`self.BP_GameInstance`)) _returnvalue)
    (bind _returnvalue_2 (`|CreateWidget` "/Game/01_Menu/Widget/Widget_MainMenu.Widget_MainMenu_C"))
    (bind _output_get (set `self.Widget_MainMenu` _returnvalue_2))
    (`UserWidget.AddToViewport` _output_get 0)
    (else
      (bind _returnvalue_3 (`|CreateWidget` "/Game/01_Menu/Widget/Widget_Pause.Widget_Pause_C"))
      (set `self.WidgetPause` _returnvalue_3))))

(event `InputAxis|Menu_UpDown` :paused true
  (params (AxisValue :type "Float (single-precision)"))
  (if (or (`/Game/02_Blueprints/BP_GameInstance.OnMenuMap` (`self.BP_GameInstance`)) (`GameplayStatics.IsGamePaused`))
    ;[1 0.7 0] Gamepad Menu
    (if (!= AxisValue 0.0)
      (message `/Game/02_Blueprints/Interfaces/BPI_MenuGamepad.SwitchInMenu_RightLeft` (select `bool` (`/Game/02_Blueprints/BP_GameInstance.OnMenuMap` (`self.BP_GameInstance`)) :`false` (`self.WidgetPause`) :`true` (`self.Widget_MainMenu`) :!type "Object Object Reference") (select `bool` (> AxisValue 0.0) :`false` -1.0 :`true` 1.0 :!type "Float (single-precision)")))
    (else
      (message `/Game/02_Blueprints/Interfaces/BPI_Character.MoveFront` (`self.BP_PlayerCharacter`) AxisValue))))

(event `InputAxis|Menu_RightLeft` :paused true
  (params (AxisValue :type "Float (single-precision)"))
  (if (or (`/Game/02_Blueprints/BP_GameInstance.OnMenuMap` (`self.BP_GameInstance`)) (`GameplayStatics.IsGamePaused`))
    ;[1 0.7 0] Gamepad Menu
    (if (!= AxisValue 0.0)
      (message `/Game/02_Blueprints/Interfaces/BPI_MenuGamepad.SwitchInMenu_UpDown` (select `bool` (`/Game/02_Blueprints/BP_GameInstance.OnMenuMap` (`self.BP_GameInstance`)) :`false` (`self.WidgetPause`) :`true` (`self.Widget_MainMenu`) :!type "Object Object Reference") (select `bool` (> AxisValue 0.0) :`false` -1.0 :`true` 1.0 :!type "Float (single-precision)")))
    (else
      (message `/Game/02_Blueprints/Interfaces/BPI_Character.MoveSide` (`self.BP_PlayerCharacter`) AxisValue))))

(event `InputAction|Validate/Jump` :paused true
  (params (Key :type "Key Structure"))
  (:`Pressed`
    (if (or (`/Game/02_Blueprints/BP_GameInstance.OnMenuMap` (`self.BP_GameInstance`)) (`GameplayStatics.IsGamePaused`))
      ;[1 0.7 0] Gamepad Menu
      (message `/Game/02_Blueprints/Interfaces/BPI_MenuGamepad.Validate` (select `bool` (`/Game/02_Blueprints/BP_GameInstance.OnMenuMap` (`self.BP_GameInstance`)) :`false` (`self.WidgetPause`) :`true` (`self.Widget_MainMenu`) :!type "Object Object Reference"))
      (else
        (message `/Game/02_Blueprints/Interfaces/BPI_Character.Event_Jump` (`self.BP_PlayerCharacter`))))))

(event `InputAction|Back` :paused true
  (params (Key :type "Key Structure"))
  (:`Pressed`
    (if (or (`/Game/02_Blueprints/BP_GameInstance.OnMenuMap` (`self.BP_GameInstance`)) (`GameplayStatics.IsGamePaused`))
      ;[1 0.7 0] Gamepad Menu
      (message `/Game/02_Blueprints/Interfaces/BPI_MenuGamepad.Back` (select `bool` (`/Game/02_Blueprints/BP_GameInstance.OnMenuMap` (`self.BP_GameInstance`)) :`false` (`self.WidgetPause`) :`true` (`self.Widget_MainMenu`) :!type "Object Object Reference")))))

(event `InputAction|Pause` :paused true
  (params (Key :type "Key Structure"))
  (bind _returnvalue (`GameplayStatics.GetPlayerController` 0))
  (bind _widgetpause (`self.WidgetPause`))
  (bind _mousemode (`/Game/02_Blueprints/BP_GameInstance.MouseMode` (`self.BP_GameInstance`)))
  ;[1 1 1] Pause Game
  (:`Pressed`
    (if (`GameplayStatics.IsGamePaused`)
      (`GameplayStatics.SetGamePaused` false)
      (`Widget.RemoveFromParent` _widgetpause)
      (`WidgetBlueprintLibrary.SetInputMode_GameOnly` _returnvalue)
      (set `PlayerController.bShowMouseCursor` _mousemode _returnvalue)
      (else
        (`GameplayStatics.SetGamePaused` true)
        (`UserWidget.AddToViewport` _widgetpause 0)
        (`WidgetBlueprintLibrary.SetInputMode_GameAndUIEx` _returnvalue)
        (set `PlayerController.bShowMouseCursor` _mousemode _returnvalue)))))

(fn `UserConstructionScript`)