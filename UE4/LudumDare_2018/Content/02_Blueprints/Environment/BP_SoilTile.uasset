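; Grid-snapped soil tile actor that holds a plant reference and registers or detaches itself as that plant changes.
; It snaps a decal preview to a 128-unit grid in construction, then snaps itself and destroys the decal on BeginPlay.
; It caches the six nearest tiles, itself included, using a hand-written recursive merge sort on a distance map.
; Neighbour-based yield logic with weighted random choice exists but is not wired to any event.
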(event `self.ReceiveBeginPlay`
  (bind (_returnvalue_x _returnvalue_y) (`KismetMathLibrary.BreakVector` (`SceneComponent.K2_GetComponentLocation` (`self.Scene`))))
  ;[0 1 0] Event BeginPlay
  (bind _asbp_player_character (cast `/Game/02_Blueprints/Character/BP_PlayerCharacter` (`GameplayStatics.GetPlayerCharacter` 0)))
  (set `self.BP_PlayerCharacter` _asbp_player_character)
  (bind _asbp_game_instance (cast `/Game/02_Blueprints/BP_GameInstance` (`GameplayStatics.GetGameInstance`)))
  (set `self.BP_GameInstance` _asbp_game_instance)
  (`self.K2_SetActorLocation` (`KismetMathLibrary.MakeVector` (`KismetMathLibrary.GridSnap_Float` _returnvalue_x 128.0) (`KismetMathLibrary.GridSnap_Float` _returnvalue_y 128.0)))
  (`ActorComponent.K2_DestroyComponent` (`self.Decal`))
  ;[1 0 1] Jason - Get Nearest Tiles
  (bind _nearesttiles (`self.getNearestTiles`))
  (set `self.nearestTiles` _nearesttiles))

(event `/Game/02_Blueprints/Interfaces/BPI_Soil.SOIL_ChangePlant`
  (params (AttachedPlant :type "/Game/02_Blueprints/Environment/BP_Plant Object Reference"))
  (bind _plant (`self.Plant`))
  (`/Engine/EditorBlueprintResources/StandardMacros.IsValid` _plant
    (:`Is Valid`
      (`/Game/02_Blueprints/Environment/BP_Plant.Remove Soil` _plant self))
    (:`Is Not Valid`
      _))
  (bind _output_get (set `self.Plant` AttachedPlant))
  (bind _asbp_soil_tile (cast `/Game/02_Blueprints/Environment/BP_SoilTile` self))
  (`/Game/02_Blueprints/Environment/BP_Plant.Add Soil` _output_get _asbp_soil_tile))

(event `/Game/02_Blueprints/Interfaces/BPI_Soil.SOIL_RemovePlant`
  (params (WithoutSprite :type Boolean))
  (bind _plant (`self.Plant`))
  (`/Engine/EditorBlueprintResources/StandardMacros.IsValid` _plant
    (:`Is Valid`
      (if (not WithoutSprite)
        (`/Game/02_Blueprints/Environment/BP_Plant.RemoveSpriteByActorRef` _plant self))
      (set `self.Plant` null))))

(fn `checkEnvironment`
  (params (seed :type "/Game/02_Blueprints/DataList/Enum_SeedsName Enum" :default "NewEnumerator5") (quantityNeeded :type Integer))
  (returns (isValidated :type Boolean))
  (locals (actualQuantity :type Integer))
  (for _array_element (`self.nearestTiles`)
    (if (`|EnumEquality` (`/Game/02_Blueprints/Environment/BP_Plant.Seed Name` (`/Game/02_Blueprints/Environment/BP_SoilTile.Plant` _array_element)) seed)
      (bind _result (`/Engine/EditorBlueprintResources/StandardMacros.IncrementInt` (`local.actualQuantity`))
        (:`  `
          (if (>= _result quantityNeeded)
            (return true))))))
  (return false))

(fn `chooseYield`
  (params (possibleYields :type "Map of /Game/02_Blueprints/DataList/Enum_SeedsName Enum to Integer" :default _))
  (returns (yieldedSeed :type "/Game/02_Blueprints/DataList/Enum_SeedsName Enum"))
  (locals (tmp :type "Array of /Game/02_Blueprints/DataList/Enum_SeedsName Enum"))
  (bind _tmp (`local.tmp`))
  (bind _keys (`BlueprintMapLibrary.Map_Keys` possibleYields))
  (bind _values (`BlueprintMapLibrary.Map_Values` possibleYields))
  (for (_array_element _array_index) _keys
    (for _ (range (+ (`|GetArrayItem` _values _array_index) 1))
      (`KismetArrayLibrary.Array_Add` (`local.tmp`) _array_element)))
  (return (`|GetArrayItem` _tmp (`KismetMathLibrary.RandomIntegerInRange` 0 (- (`KismetArrayLibrary.Array_Length` _tmp) 1)))))

(fn `getNearestTiles`
  (returns (nearestTiles :type "Array of /Game/02_Blueprints/Environment/BP_SoilTile Object Reference"))
  (locals (closest :type "Float (double-precision)") (tiles :type "Map of /Game/02_Blueprints/Environment/BP_SoilTile Object Reference to Float (double-precision)"))
  (bind _outactors (`GameplayStatics.GetAllActorsOfClass` "BP_SoilTile_C"))
  (for _array_element _outactors
    (`BlueprintMapLibrary.Map_Add` (`local.tiles`) _array_element (`self.GetDistanceTo` _array_element)))
  (bind _result (`self.mergeSort` (`local.tiles`)))
  (bind _keys (`BlueprintMapLibrary.Map_Keys` _result))
  (for _index (range 6 (`KismetArrayLibrary.Array_Length` _keys))
    (`BlueprintMapLibrary.Map_Remove` (`local.tiles`) (`|GetArrayItem` _keys _index)))
  (bind _keys_2 (`BlueprintMapLibrary.Map_Keys` (`local.tiles`)))
  (return _keys_2))

(fn `merge`
  (params (left :type "Map of /Game/02_Blueprints/Environment/BP_SoilTile Object Reference to Float (double-precision)") (right :type "Map of /Game/02_Blueprints/Environment/BP_SoilTile Object Reference to Float (double-precision)"))
  (returns (result :type "Map of /Game/02_Blueprints/Environment/BP_SoilTile Object Reference to Float (double-precision)"))
  (locals (resultMap :type "Map of /Game/02_Blueprints/Environment/BP_SoilTile Object Reference to Float (double-precision)"))
  (bind _returnvalue (> (`BlueprintMapLibrary.Map_Length` left) 0))
  (bind _returnvalue_2 (> (`BlueprintMapLibrary.Map_Length` right) 0))
  (while (and _returnvalue _returnvalue_2)
    (bind _values (`BlueprintMapLibrary.Map_Values` left))
    (bind _values_2 (`BlueprintMapLibrary.Map_Values` right))
    (if (<= (`|GetArrayItem` _values) (`|GetArrayItem` _values_2))
      (bind _keys (`BlueprintMapLibrary.Map_Keys` left))
      (bind _values_3 (`BlueprintMapLibrary.Map_Values` left))
      (bind _output (`|GetArrayItem` _keys))
      (`BlueprintMapLibrary.Map_Add` (`local.resultMap`) _output (`|GetArrayItem` _values_3))
      (`BlueprintMapLibrary.Map_Remove` left _output)
      (else
        (bind _keys_2 (`BlueprintMapLibrary.Map_Keys` right))
        (bind _values_4 (`BlueprintMapLibrary.Map_Values` right))
        (bind _output_2 (`|GetArrayItem` _keys_2))
        (`BlueprintMapLibrary.Map_Add` (`local.resultMap`) _output_2 (`|GetArrayItem` _values_4))
        (`BlueprintMapLibrary.Map_Remove` right _output_2))))
  (if _returnvalue
    (bind _keys_3 (`BlueprintMapLibrary.Map_Keys` left))
    (bind _values_5 (`BlueprintMapLibrary.Map_Values` left))
    (for (_array_element _array_index) _keys_3
      (`BlueprintMapLibrary.Map_Add` (`local.resultMap`) _array_element (`|GetArrayItem` _values_5 _array_index))))
  (if _returnvalue_2
    (bind _keys_4 (`BlueprintMapLibrary.Map_Keys` right))
    (bind _values_6 (`BlueprintMapLibrary.Map_Values` right))
    (for (_array_element_2 _array_index_2) _keys_4
      (`BlueprintMapLibrary.Map_Add` (`local.resultMap`) _array_element_2 (`|GetArrayItem` _values_6 _array_index_2))))
  (return (`local.resultMap`)))

(fn `mergeSort`
  (params (map :type "Map of /Game/02_Blueprints/Environment/BP_SoilTile Object Reference to Float (double-precision)"))
  (returns (result :type "Map of /Game/02_Blueprints/Environment/BP_SoilTile Object Reference to Float (double-precision)"))
  (locals (middleIndex :type Integer) (left :type "Map of /Game/02_Blueprints/Environment/BP_SoilTile Object Reference to Float (double-precision)") (right :type "Map of /Game/02_Blueprints/Environment/BP_SoilTile Object Reference to Float (double-precision)") (firstIndex :type Integer))
  (bind _returnvalue (`BlueprintMapLibrary.Map_Length` map))
  (bind _right (`local.right`))
  (if (<= _returnvalue 1)
    (return map)
    (else
      (bind _output_get (set `local.middleIndex` (/ _returnvalue 2)))
      (for _index (range (`local.firstIndex`) _output_get)
        (bind _keys (`BlueprintMapLibrary.Map_Keys` map))
        (bind _values (`BlueprintMapLibrary.Map_Values` map))
        (`BlueprintMapLibrary.Map_Add` (`local.left`) (`|GetArrayItem` _keys _index) (`|GetArrayItem` _values _index)))
      (for _index_2 (range (`local.middleIndex`) (+ (`BlueprintMapLibrary.Map_Length` map) 1))
        (bind _keys_2 (`BlueprintMapLibrary.Map_Keys` map))
        (bind _values_2 (`BlueprintMapLibrary.Map_Values` map))
        (`BlueprintMapLibrary.Map_Add` (`local.right`) (`|GetArrayItem` _keys_2 _index_2) (`|GetArrayItem` _values_2 _index_2)))
      (bind _result (`self.mergeSort` (`local.left`)))
      (set `local.left` _result)
      (bind _result_2 (`self.mergeSort` (`local.right`)))
      (set `local.right` _result_2)
      (bind _values_3 (`BlueprintMapLibrary.Map_Values` (`local.left`)))
      (bind _values_4 (`BlueprintMapLibrary.Map_Values` (`local.right`)))
      (if (<= (`|GetArrayItem` _values_3 (- (`KismetArrayLibrary.Array_Length` _values_3) 1)) (`|GetArrayItem` _values_4))
        (bind _keys_3 (`BlueprintMapLibrary.Map_Keys` _right))
        (bind _values_5 (`BlueprintMapLibrary.Map_Values` _right))
        (for (_array_element _array_index) _keys_3
          (`BlueprintMapLibrary.Map_Add` (`local.left`) _array_element (`|GetArrayItem` _values_5 _array_index)))
        (return (`local.left`))
        (else
          (`self.merge` (`local.left`) (`local.right`))
          (return))))))

(fn `SOIL_GetPlant`
  (returns (SeedName :type Name) (PlantStruct :type "/Game/02_Blueprints/DataList/Struct_Objects Structure"))
  (bind _plant (`self.Plant`))
  (`/Engine/EditorBlueprintResources/StandardMacros.IsValid` _plant
    (:`Is Valid`
      (return (`KismetStringLibrary.Conv_StringToName` (`|GetEnumeratorNameAsString` (`/Game/02_Blueprints/Environment/BP_Plant.Seed Name` _plant))) (`/Game/02_Blueprints/Environment/BP_Plant.PlantStruct` _plant)))
    (:`Is Not Valid`
      (return "None"))))

(fn `UserConstructionScript`
  (bind (_returnvalue_x _returnvalue_y) (`KismetMathLibrary.BreakVector` (`SceneComponent.K2_GetComponentLocation` (`self.Scene`))))
  (`SceneComponent.K2_SetWorldLocation` (`self.Decal`) (`KismetMathLibrary.MakeVector` (`KismetMathLibrary.GridSnap_Float` _returnvalue_x 128.0) (`KismetMathLibrary.GridSnap_Float` _returnvalue_y 128.0)) false false))