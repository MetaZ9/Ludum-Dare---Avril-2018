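; Plant actor that occupies soil tiles, with a seed sprite and a growth ("Pousse") behavior defined by its seed type.
; BeginPlay reads the seed's DataT_Objects row, adds the matching growth component (size x2, eat neighbor, move, extend, push neighbors), then after a brief delay registers with the soil that component finds.
; Helpers add, move and remove sprites, matching them to soils by XY proximity.
; The plant destroys itself when its soils or sprites run out.
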(event `self.ReceiveBeginPlay`
  (`|ExecutionSequence`
    (:`then_0`
      ;[1 1 1] Set Struct variable and Pousse Effect
      (bind _returnvalue (`|GetDataTableRow` "/Game/02_Blueprints/DataList/DataT_Objects.DataT_Objects" (`KismetStringLibrary.Conv_StringToName` (`|GetEnumeratorNameAsString` (`self.Seed Name`))))
        (:`then`
          (set `self.PlantStruct` _returnvalue)
          (switch `/Game/02_Blueprints/DataList/Enum_PousseEffect` (`.PousseEffect_14_0DFFAB2947503EA9EDFF829BD4616795` (break `/Game/02_Blueprints/DataList/Struct_Objects` (`self.PlantStruct`)))
            (:`NewEnumerator1`
              (bind _returnvalue_2 (`AddComponent|NODE_AddSC_Pousse_Taille_x2-0` :`Owner` null))
              (set `self.PousseEffect` _returnvalue_2))
            (:`NewEnumerator2`
              (bind _returnvalue_3 (`AddComponent|NODE_AddSC_Pousse_EatNear-0` :`Owner` self))
              (set `self.PousseEffect` _returnvalue_3))
            (:`NewEnumerator3`
              (bind _returnvalue_4 (`AddComponent|NODE_AddSC_Pousse_Deplacement-1` :`Owner` self))
              (set `self.PousseEffect` _returnvalue_4))
            (:`NewEnumerator4`
              (bind _returnvalue_5 (`AddComponent|NODE_AddSC_Pousse_Extend-0` :`Owner` self))
              (set `self.PousseEffect` _returnvalue_5))
            (:`NewEnumerator6`
              (bind _returnvalue_6 (`AddComponent|NODE_AddSC_Pousse_Souffle-0` :`Owner` self))
              (set `self.PousseEffect` _returnvalue_6))))
        (:`RowNotFound`
          (`KismetSystemLibrary.PrintString` "Failed To Find RightName" true true (struct :`R` 1.0 :`A` 1.0) 25.0))))
    (:`then_1`
      ;[1 1 1] Set Location
      (`KismetSystemLibrary.Delay` 0.1)
      (bind _soilfind (`/Game/02_Blueprints/Components/SC_0Pousse.FindSoil_LesserRange` (`self.PousseEffect`) (`self.DefaultSceneRoot`)))
      (message `/Game/02_Blueprints/Interfaces/BPI_Soil.SOIL_ChangePlant` _soilfind self)
      (`self.AddSprite` _soilfind))))

(event `Add Soil`
  (params (`Soil Ref` :type "/Game/02_Blueprints/Environment/BP_SoilTile Object Reference (by ref)"))
  (`KismetArrayLibrary.Array_AddUnique` (`self.Soil`) `Soil Ref`))

(event `Remove Soil`
  (params (`Soil Ref` :type "/Game/02_Blueprints/Environment/BP_SoilTile Object Reference"))
  (bind _soil (`self.Soil`))
  (bind _returnvalue (`KismetArrayLibrary.Array_Find` _soil `Soil Ref`))
  (if (!= _returnvalue -1)
    (`self.RemoveSpriteByActorRef` `Soil Ref`)
    (`KismetArrayLibrary.Array_Remove` _soil _returnvalue)
    (if (== (`KismetArrayLibrary.Array_Length` (`self.Soil`)) 0)
      (`self.K2_DestroyActor`))))

(fn `AddSprite`
  (params (Actor :type "Actor Object Reference"))
  (bind _sprites (`self.Sprites`))
  (bind (_taille _pousseeffect _effect _goldeneffect _goldeneffectprobability _life _imgseed) (break `/Game/02_Blueprints/DataList/Struct_Objects` (`self.PlantStruct`)))
  (bind _returnvalue (`AddComponent|NODE_AddPaperSpriteComponent-0` :`RelativeTransform` (`KismetMathLibrary.MakeTransform` (0.0 0.0 25.0) (struct :`Yaw` 90.0 :`Roll` 90.0))))
  (`SceneComponent.K2_SetWorldLocation` _returnvalue (+ (`self.K2_GetActorLocation` Actor) (0.0 0.0 25.0)) false false)
  (`KismetArrayLibrary.Array_Set` _sprites (+ (`KismetArrayLibrary.Array_LastIndex` _sprites) 1) _returnvalue true)
  (`PaperSpriteComponent.SetSprite` _returnvalue _imgseed)
  (`KismetSystemLibrary.PrintString` (`KismetStringLibrary.Concat_StrStr` "Img : " (`KismetSystemLibrary.GetDisplayName` _imgseed)) false true (struct :`R` 1.0 :`B` 0.025802 :`A` 1.0) 25.0))

(fn `FindIndexByActor`
  (params (Actor :type "Actor Object Reference"))
  (returns (IndexFind :type Integer) (PaperRef :type "PaperSpriteComponent Object Reference"))
  (locals (IndexRef :type Integer))
  (bind (_returnvalue_x _returnvalue_y) (`KismetMathLibrary.BreakVector` (`self.K2_GetActorLocation` Actor)))
  (bind _indexref (`local.IndexRef`))
  (set `local.IndexRef` -1)
  (for (_array_element _array_index) (`self.Sprites`)
    (`/Engine/EditorBlueprintResources/StandardMacros.IsValid` _array_element
      (:`Is Valid`
        (bind (_returnvalue_x_2 _returnvalue_y_2) (`KismetMathLibrary.BreakVector` (`SceneComponent.K2_GetComponentLocation` _array_element)))
        (if (<= (+ (`KismetMathLibrary.Abs` (- _returnvalue_x_2 _returnvalue_x)) (`KismetMathLibrary.Abs` (- _returnvalue_y_2 _returnvalue_y))) 30.0)
          (set `local.IndexRef` _array_index)
          (break)))))
  (return _indexref (`|GetArrayItem` (`self.Sprites`) _indexref)))

(fn `MoveTo`
  (params (Actor :type "Actor Object Reference"))
  (locals (Value :type "IntVector Structure"))
  (bind (_value_x _value_y) (break `IntVector` (`local.Value`)))
  (bind (_value_x_2 _value_y_2) (break `IntVector` (`local.Value`)))
  (`self.K2_SetActorLocation` (`self.K2_GetActorLocation` Actor) false true)
  (for (_array_element _array_index) (`self.Sprites`)
    (`SceneComponent.K2_SetWorldLocation` _array_element (+ (`self.K2_GetActorLocation`) (`KismetMathLibrary.MakeVector` (* _value_x_2 128.0) (* _value_y_2 128.0) 25.0)) false false)
    (if (not (== _array_index 0))
      (bind _returnvalue (!= (mod _array_index 2) 0))
      (set `local.Value` (make `IntVector` (select `bool` _returnvalue :`false` (+ _value_x 1) :`true` _value_x) (select `bool` _returnvalue :`false` _value_y :`true` (+ _value_y 1)))))))

(fn `MoveToByIndex`
  (params (Index :type Integer) (Actor :type "Actor Object Reference"))
  (locals (Value :type "IntVector Structure"))
  (bind _output (`|GetArrayItem` (`self.Sprites`) Index))
  (if (and (`KismetSystemLibrary.IsValid` _output) (`KismetSystemLibrary.IsValid` Actor))
    (`SceneComponent.K2_SetWorldLocation` _output (+ (`self.K2_GetActorLocation` Actor) (0.0 0.0 25.0)) false false)))

(fn `RemoveSprite_ByIndex`
  (params (Index :type Integer))
  (bind _output (`|GetArrayItem` (`self.Sprites`) Index))
  (`/Engine/EditorBlueprintResources/StandardMacros.IsValid` _output
    (:`Is Valid`
      (`ActorComponent.K2_DestroyComponent` _output)
      (`KismetArrayLibrary.Array_RemoveItem` (`self.Sprites`) _output)
      (if (== (`KismetArrayLibrary.Array_Length` (`self.Sprites`)) 0)
        (`self.K2_DestroyActor`)))))

(fn `RemoveSpriteByActorRef`
  (params (Actor :type "Actor Object Reference"))
  (bind (_returnvalue_x _returnvalue_y) (`KismetMathLibrary.BreakVector` (`self.K2_GetActorLocation` Actor)))
  (for _array_element (`self.Sprites`)
    (`/Engine/EditorBlueprintResources/StandardMacros.IsValid` _array_element
      (:`Is Valid`
        (bind (_returnvalue_x_2 _returnvalue_y_2) (`KismetMathLibrary.BreakVector` (`SceneComponent.K2_GetComponentLocation` _array_element)))
        (if (<= (+ (`KismetMathLibrary.Abs` (- _returnvalue_x_2 _returnvalue_x)) (`KismetMathLibrary.Abs` (- _returnvalue_y_2 _returnvalue_y))) 5.0)
          (`KismetSystemLibrary.PrintString` "Destroy")
          (`ActorComponent.K2_DestroyComponent` _array_element)
          (`KismetArrayLibrary.Array_RemoveItem` (`self.Sprites`) _array_element)
          (break)))))
  (if (== (`KismetArrayLibrary.Array_Length` (`self.Sprites`)) 0)
    (`self.K2_DestroyActor`)))

(fn `UserConstructionScript`)