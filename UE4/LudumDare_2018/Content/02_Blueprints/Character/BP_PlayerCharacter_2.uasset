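; Player character with flipbook sprites that walks, runs, farms soil tiles and shoots bullets along a facing arrow.
; Movement axes choose the sprite and facing; mouse or pad input, per the GameInstance's MouseMode, pans a clamped spring arm, with a timeline for recentring.
; A front collision box targets soil to harvest into the inventory widget or plant a random seed.
; Damage lowers GameInstance life, showing a death widget and returning to the main menu at zero.
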(event `self.ReceiveBeginPlay`
  ;[0 1 0] Event BeginPlay
  (bind _asbp_game_instance (cast `/Game/02_Blueprints/BP_GameInstance` (`GameplayStatics.GetGameInstance`)))
  (set `self.BP_GameInstance` _asbp_game_instance)
  (bind _returnvalue (`|CreateWidget` "/Game/02_Blueprints/Widget/Widget_Inventaire.Widget_Inventaire_C"))
  (bind _output_get (set `self.Widget_Inventaire` _returnvalue))
  (`UserWidget.AddToViewport` _output_get 0))

(event `InputAxis|Camera_MoveSide_Mouse`
  (params (AxisValue :type "Float (single-precision)"))
  (bind (_camera_minvalue_x _camera_minvalue_y) (`KismetMathLibrary.BreakVector2D` (`self.Camera_MinValue`)))
  (bind (_camera_maxvalue_x _camera_maxvalue_y) (`KismetMathLibrary.BreakVector2D` (`self.Camera_MaxValue`)))
  (bind (_camera_minvalue_x_2 _camera_minvalue_y_2) (`KismetMathLibrary.BreakVector2D` (`self.Camera_MinValue`)))
  (bind (_camera_maxvalue_x_2 _camera_maxvalue_y_2) (`KismetMathLibrary.BreakVector2D` (`self.Camera_MaxValue`)))
  (bind (_returnvalue_x _returnvalue_y) (`KismetMathLibrary.BreakVector` (`SceneComponent.K2_GetComponentLocation` (`self.CharacterFlipbook`))))
  (bind (_returnvalue_x_2 _returnvalue_y_2 _returnvalue_z) (`KismetMathLibrary.BreakVector` (`SceneComponent.K2_GetComponentLocation` (`self.SpringArm`))))
  (bind (_returnvalue_x_3 _returnvalue_y_3) (`KismetMathLibrary.BreakVector` (`SceneComponent.K2_GetComponentLocation` (`self.CharacterFlipbook`))))
  (bind (_returnvalue_x_4 _returnvalue_y_4 _returnvalue_z_2) (`KismetMathLibrary.BreakVector` (`SceneComponent.K2_GetComponentLocation` (`self.SpringArm`))))
  (bind _mousemode (`/Game/02_Blueprints/BP_GameInstance.MouseMode` (`self.BP_GameInstance`)))
  ;[0 1 1] Camera Move
  (if _mousemode
    (`|ExecutionSequence` :!label _label
      (:`then_0`
        (bind (_direction _newtrack_0) (`Timeline|Timeline_1` :!via `Stop` :!label _label_2)
          (:`Update`
            (`SceneComponent.K2_SetWorldLocation` (`self.SpringArm`) (`KismetMathLibrary.MakeVector` (`KismetMathLibrary.FClamp` (`KismetMathLibrary.Lerp` _returnvalue_x_2 _returnvalue_x _newtrack_0) _camera_minvalue_x _camera_maxvalue_x) (`KismetMathLibrary.FClamp` (`KismetMathLibrary.Lerp` _returnvalue_y_2 _returnvalue_y _newtrack_0) _camera_minvalue_y _camera_maxvalue_y) _returnvalue_z) false false))))
      (:`then_1`
        (bind _returnvalue (select `bool` _mousemode :`false` (stale `InputAxis|Camera_MoveSide_Pad` AxisValue) :`true` AxisValue))
        (`SceneComponent.K2_SetWorldLocation` (`self.SpringArm`) (`KismetMathLibrary.MakeVector` _returnvalue_x_4 (`KismetMathLibrary.FClamp` (`KismetMathLibrary.FClamp` (+ (* _returnvalue 10.0) _returnvalue_y_4) (+ _returnvalue_y_3 -1000.0) (+ _returnvalue_y_3 1000.0)) _camera_minvalue_y_2 _camera_maxvalue_y_2) _returnvalue_z_2) false false))
      (:`then_2`
        (goto _label_3 :!via `Reset`))
      (:`then_3`
        (if (not (not (and (== _returnvalue 0.0) (== (select `bool` _mousemode :`false` (stale `InputAxis|Camera_MoveUpDown_Pad` AxisValue) :`true` (stale `InputAxis|Camera_MoveUpDown_Mouse` AxisValue)) 0.0))))
          (`/Engine/EditorBlueprintResources/StandardMacros.DoOnce` false :!label _label_3
            (:`Completed`
              (goto _label_2 :!via `PlayFromStart`))))))))

(event `/Game/02_Blueprints/Interfaces/BPI_Character.MoveFront`
  (params (MoveFront :type "Float (single-precision)"))
  ;[0 0.5 1] Character Move
  (bind _returnvalue (select `bool` (`/Game/02_Blueprints/BP_GameInstance.MouseMode` (`self.BP_GameInstance`)) :`false` MoveFront :`true` (stale `InputAxis|Move_Front` AxisValue)))
  (bind _returnvalue_2 (select `bool` (`/Game/02_Blueprints/BP_GameInstance.MouseMode` (`self.BP_GameInstance`)) :`false` (stale `/Game/02_Blueprints/Interfaces/BPI_Character.MoveSide` MoveSide) :`true` (stale `InputAxis|Move_Side` AxisValue)))
  (`ActorComponent.SetActive` (`self.Audio`) (or (!= _returnvalue 0.0) (!= _returnvalue_2 0.0)) false :!label _label_4)
  (bind _returnvalue_3 (!= _returnvalue 0.0))
  (set `self.IsWalking?` (or _returnvalue_3 (!= _returnvalue_2 0.0)))
  (`self.AddMovementInput` (1.0 0.0 0.0) _returnvalue)
  (if (not (< (`KismetMathLibrary.Abs` _returnvalue) (`KismetMathLibrary.Abs` _returnvalue_2)))
    (`/Engine/EditorBlueprintResources/StandardMacros.DoOnce` false :!label _label_5
      (:`Completed`
        (bind _returnvalue_4 (> _returnvalue 0.0))
        (`PaperFlipbookComponent.SetFlipbook` (`self.CharacterFlipbook`) (select `bool` _returnvalue_4 :`false` "/Game/05_GA/Assets/MainCharacter/FlipBook/FlipBook_mainChara_WalkFront.FlipBook_mainChara_WalkFront" :`true` "/Game/05_GA/Assets/MainCharacter/FlipBook/FlipBook_mainChara_WalkBack.FlipBook_mainChara_WalkBack" :!type "PaperFlipbook Object Reference"))
        (if _returnvalue_3
          (`SceneComponent.K2_SetRelativeRotation` (`self.Arrow1`) (`KismetMathLibrary.MakeRotator` 0.0 0.0 (select `bool` _returnvalue_4 :`false` -180.0 :!type "Float (single-precision)")) false false))))
    (else
      (goto _label_5 :!via `Reset`))))

(event `InputAxis|Camera_MoveSide_Pad`
  (params (AxisValue :type "Float (single-precision)"))
  ;[0 1 1] Camera Move
  (if (not (`/Game/02_Blueprints/BP_GameInstance.MouseMode` (`self.BP_GameInstance`)))
    (goto _label)))

(event `InputAxis|Move_Front`
  (params (AxisValue :type "Float (single-precision)"))
  ;[0 0.5 1] Character Move
  (goto _label_4))

(event `/Game/02_Blueprints/Interfaces/BPI_Character.MoveSide`
  (params (MoveSide :type "Float (single-precision)"))
  ;[0 0.5 1] Character Move
  (bind _returnvalue (select `bool` (`/Game/02_Blueprints/BP_GameInstance.MouseMode` (`self.BP_GameInstance`)) :`false` (stale `/Game/02_Blueprints/Interfaces/BPI_Character.MoveFront` MoveFront) :`true` (stale `InputAxis|Move_Front` AxisValue)))
  (bind _returnvalue_2 (select `bool` (`/Game/02_Blueprints/BP_GameInstance.MouseMode` (`self.BP_GameInstance`)) :`false` MoveSide :`true` (stale `InputAxis|Move_Side` AxisValue)))
  (`ActorComponent.SetActive` (`self.Audio`) (or (!= _returnvalue 0.0) (!= _returnvalue_2 0.0)) false :!label _label_6)
  (`self.AddMovementInput` (0.0 1.0 0.0) _returnvalue_2)
  (if (< (`KismetMathLibrary.Abs` _returnvalue) (`KismetMathLibrary.Abs` _returnvalue_2))
    (`/Engine/EditorBlueprintResources/StandardMacros.DoOnce` false :!label _label_7
      (:`Completed`
        (`PaperFlipbookComponent.SetFlipbook` (`self.CharacterFlipbook`) "/Game/05_GA/Assets/MainCharacter/FlipBook/FlipBook_mainChara_walk_side.FlipBook_mainChara_walk_side")))
    (else
      (`|ExecutionSequence`
        (:`then_0`
          (goto _label_7 :!via `Reset`))
        (:`then_1`
          _))))
  (if (!= _returnvalue_2 0.0)
    (bind _returnvalue_3 (select `bool` (>= _returnvalue_2 0.0) :`false` 180.0 :!type "Float (single-precision)"))
    (`SceneComponent.K2_SetRelativeRotation` (`self.CharacterFlipbook`) (`KismetMathLibrary.MakeRotator` -90.0 _returnvalue_3 90.0) false false)
    (`SceneComponent.K2_SetRelativeRotation` (`self.Arrow1`) (`KismetMathLibrary.MakeRotator` 0.0 _returnvalue_3 90.0) false false)))

(event `InputAxis|Move_Side`
  (params (AxisValue :type "Float (single-precision)"))
  ;[0 0.5 1] Character Move
  (goto _label_6))

(event `InputAction|Run`
  (params (Key :type "Key Structure"))
  (bind _charactermovement (`self.CharacterMovement`))
  ;[0 0.5 1] Character Move
  (:`Pressed`
    (if (`self.IsWalking?`)
      (set `CharacterMovementComponent.MaxWalkSpeed` 1200.0 _charactermovement)))
  (:`Released`
    (set `CharacterMovementComponent.MaxWalkSpeed` 600.0 _charactermovement)))

(event `InputAxis|Camera_MoveUpDown_Mouse`
  (params (AxisValue :type "Float (single-precision)"))
  (bind _camera_minvalue_x (`KismetMathLibrary.BreakVector2D` (`self.Camera_MinValue`)))
  (bind _camera_maxvalue_x (`KismetMathLibrary.BreakVector2D` (`self.Camera_MaxValue`)))
  (bind (_returnvalue_x _returnvalue_y _returnvalue_z) (`KismetMathLibrary.BreakVector` (`SceneComponent.K2_GetComponentLocation` (`self.SpringArm`))))
  (bind _returnvalue_x_2 (`KismetMathLibrary.BreakVector` (`SceneComponent.K2_GetComponentLocation` (`self.CapsuleComponent`))))
  (bind _mousemode (`/Game/02_Blueprints/BP_GameInstance.MouseMode` (`self.BP_GameInstance`)))
  ;[0 1 1] Camera Move
  (if _mousemode
    (`SceneComponent.K2_SetWorldLocation` (`self.SpringArm`) (`KismetMathLibrary.MakeVector` (`KismetMathLibrary.FClamp` (`KismetMathLibrary.FClamp` (+ (* (select `bool` _mousemode :`false` (stale `InputAxis|Camera_MoveUpDown_Pad` AxisValue) :`true` AxisValue) 10.0) _returnvalue_x) (+ _returnvalue_x_2 -500.0) (+ _returnvalue_x_2 500.0)) _camera_minvalue_x _camera_maxvalue_x) _returnvalue_y _returnvalue_z) false false :!label _label_8)))

(event `InputAxis|Camera_MoveUpDown_Pad`
  (params (AxisValue :type "Float (single-precision)"))
  ;[0 1 1] Camera Move
  (if (not (`/Game/02_Blueprints/BP_GameInstance.MouseMode` (`self.BP_GameInstance`)))
    (goto _label_8)))

(event `self.FrontCollisionBox.OnComponentBeginOverlap`
  (params (OverlappedComponent :type "PrimitiveComponent Object Reference") (OtherActor :type "Actor Object Reference") (OtherComp :type "PrimitiveComponent Object Reference") (OtherBodyIndex :type Integer) (bFromSweep :type Boolean) (SweepResult :type "HitResult Structure (by ref)"))
  ;[1 1 1] Events Collect
  (if (== (`GameplayStatics.GetObjectClass` OtherActor) "/Game/02_Blueprints/Environment/BP_SoilTile.BP_SoilTile_C")
    (set `self.SomethingIn?` true)
    (set `self.ObjectInBox` OtherActor)))

(event `self.FrontCollisionBox.OnComponentEndOverlap`
  (params (OverlappedComponent :type "PrimitiveComponent Object Reference") (OtherActor :type "Actor Object Reference") (OtherComp :type "PrimitiveComponent Object Reference") (OtherBodyIndex :type Integer))
  ;[1 1 1] Events Collect
  (if (== OtherActor (`self.ObjectInBox`))
    (set `self.SomethingIn?` false)))

(event `InputAction|GetObject`
  (params (Key :type "Key Structure"))
  (bind _objectinbox (`self.ObjectInBox`))
  (bind _seeds_number (`self.Seeds_Number`))
  ;[1 1 1] Events Collect
  (:`Pressed`
    (if (`self.SomethingIn?`) :!label _label_9
      (`GameplayStatics.PlaySoundAtLocation` "/Game/05_Sound/crop_harvesting_sfx.crop_harvesting_sfx" (`self.K2_GetActorLocation`))
      (bind _seedname (message `/Game/02_Blueprints/Interfaces/BPI_Soil.SOIL_GetPlant` _objectinbox))
      (if (!= _seedname "None")
        (bind _outrownames (`DataTableFunctionLibrary.GetDataTableRowNames` "/Game/02_Blueprints/DataList/DataT_Objects.DataT_Objects"))
        (bind _returnvalue (`KismetArrayLibrary.Array_Find` _outrownames _seedname))
        (`KismetArrayLibrary.Array_Set` _seeds_number _returnvalue (+ (`|GetArrayItem` _seeds_number _returnvalue) 1))
        (message `/Game/02_Blueprints/Interfaces/BPI_Inventaire.NewElementInventaire` (`self.Widget_Inventaire`) _seedname)
        (message `/Game/02_Blueprints/Interfaces/BPI_Soil.SOIL_RemovePlant` _objectinbox false)
        (`KismetSystemLibrary.PrintString` "Add to inventory" true true (struct :`R` 1.0 :`G` 0.681906 :`A` 1.0))
        (else
          (`|SpawnActorFromClass` "/Game/02_Blueprints/Environment/BP_Plant.BP_Plant_C" (`KismetMathLibrary.MakeTransform` (+ (`self.K2_GetActorLocation` _objectinbox) (0.0 0.0 25.0))) "Undefined" "OverrideRootScale" null (cast `/Game/02_Blueprints/DataList/Enum_SeedsName` (`KismetMathLibrary.Conv_IntToByte` (`KismetMathLibrary.RandomIntegerInRange` 0 18))) null)
          (`KismetSystemLibrary.PrintString` "Plantée !" true true (struct :`R` 1.0 :`G` 0.916201 :`A` 1.0)))))))

(event `/Game/02_Blueprints/Interfaces/BPI_Character.Event_Jump`
  ;[1 1 1] Events Collect
  (goto _label_9))

(event `/Game/02_Blueprints/Interfaces/BPI_Character.Degats`
  (params (Mob_Degats :type "Float (single-precision)"))
  (bind _bp_gameinstance (`self.BP_GameInstance`))
  (bind _output_get (set `/Game/02_Blueprints/BP_GameInstance.Character_Life` (- (`/Game/02_Blueprints/BP_GameInstance.Character_Life` _bp_gameinstance) Mob_Degats) _bp_gameinstance))
  (if (<= _output_get 0.0)
    (bind _returnvalue (`|CreateWidget` "/Game/02_Blueprints/Widget/Widget_Death.Widget_Death_C"))
    (`UserWidget.AddToViewport` _returnvalue 0)
    (`KismetSystemLibrary.Delay` 3.0)
    (`GameplayStatics.OpenLevel` "Map_MainMenu")
    (set `/Game/02_Blueprints/BP_GameInstance.OnMenuMap` true (`self.BP_GameInstance`))
    (else
      (message `/Game/02_Blueprints/Interfaces/BPI_Character.LessLife` (`self.Widget_Inventaire`)))))

(event `InputAction|Attack`
  (params (Key :type "Key Structure"))
  (bind _arrow1 (`self.Arrow1`))
  (:`Pressed`
    (bind _returnvalue (`|SpawnActorFromClass` "/Game/02_Blueprints/Character/BP_Bullet.BP_Bullet_C" (`SceneComponent.K2_GetComponentToWorld` _arrow1) "AlwaysSpawn" "OverrideRootScale" null null))
    (set `MovementComponent.Velocity` (* (`SceneComponent.GetForwardVector` _arrow1) 400.0) (`/Game/02_Blueprints/Character/BP_Bullet.ProjectileMovement` _returnvalue))))

(fn `UserConstructionScript`)