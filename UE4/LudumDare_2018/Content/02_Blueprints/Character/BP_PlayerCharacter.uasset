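; Player character Blueprint with flipbook visuals: walks with direction-based animation, runs while held, shoots bullets and collects from overlapped objects.
; Axis input drives movement and clamped spring-arm camera offsets, with mouse or pad chosen by the GameInstance's MouseMode and a timeline rescaling the offset.
; A front collision box supplies the object to collect, whose seed name goes to the inventory widget.
; Damage lowers GameInstance life, showing a death widget and returning to the main menu at zero.
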(event `self.ReceiveBeginPlay`
  ;[0 1 0] Event BeginPlay
  (bind _asbp_game_instance (cast `/Game/02_Blueprints/BP_GameInstance` (`GameplayStatics.GetGameInstance`)))
  (set `self.BP_GameInstance` _asbp_game_instance)
  (bind _returnvalue (`|CreateWidget` "/Game/02_Blueprints/Widget/Widget_Inventaire.Widget_Inventaire_C"))
  (bind _output_get (set `self.Widget_Inventaire` _returnvalue))
  (`UserWidget.AddToViewport` _output_get 0))

(event `/Game/02_Blueprints/Interfaces/BPI_Character.MoveFront`
  (params (MoveFront :type "Float (single-precision)"))
  ;[0 0.5 1] Character Move
  (bind _returnvalue (select `bool` (`/Game/02_Blueprints/BP_GameInstance.MouseMode` (`self.BP_GameInstance`)) :`false` MoveFront :`true` (stale `InputAxis|Move_Front` AxisValue)))
  (bind _returnvalue_2 (select `bool` (`/Game/02_Blueprints/BP_GameInstance.MouseMode` (`self.BP_GameInstance`)) :`false` (stale `/Game/02_Blueprints/Interfaces/BPI_Character.MoveSide` MoveSide) :`true` (stale `InputAxis|Move_Side` AxisValue)))
  (set `self.IsWalking?` (or (!= _returnvalue 0.0) (!= _returnvalue_2 0.0)) :!label _label)
  (`self.AddMovementInput` (1.0 0.0 0.0) _returnvalue)
  (if (not (not (< (`KismetMathLibrary.Abs` _returnvalue) (`KismetMathLibrary.Abs` _returnvalue_2))))
    (`/Engine/EditorBlueprintResources/StandardMacros.DoOnce` false :!via `Reset`
      (:`Completed`
        _)))
  (`PaperFlipbookComponent.SetFlipbook` (`self.CharacterFlipbook`) (select `bool` (> _returnvalue 0.0) :`false` "/Game/05_GA/Assets/MainCharacter/FlipBook/FlipBook_mainChara_WalkFront.FlipBook_mainChara_WalkFront" :`true` "/Game/05_GA/Assets/MainCharacter/FlipBook/FlipBook_mainChara_WalkBack.FlipBook_mainChara_WalkBack" :!type "PaperFlipbook Object Reference")))

(event `InputAxis|Camera_MoveSide_Mouse`
  (params (AxisValue :type "Float (single-precision)"))
  (bind _springarm (`self.SpringArm`))
  (bind (_relativelocation_x _relativelocation_y) (`KismetMathLibrary.BreakVector` (`SceneComponent.RelativeLocation` _springarm)))
  (bind (_relativelocation_x_2 _relativelocation_y_2 _relativelocation_z) (`KismetMathLibrary.BreakVector` (`SceneComponent.RelativeLocation` _springarm)))
  (bind _mousemode (`/Game/02_Blueprints/BP_GameInstance.MouseMode` (`self.BP_GameInstance`)))
  ;[0 1 1] Camera Move
  (if _mousemode
    (bind _returnvalue (select `bool` _mousemode :`false` (stale `InputAxis|Camera_MoveSide_Pad` AxisValue) :`true` AxisValue))
    (if (not (and (== _returnvalue 0.0) (== (select `bool` _mousemode :`false` (stale `InputAxis|Camera_MoveUpDown_Pad` AxisValue) :`true` (stale `InputAxis|Camera_MoveUpDown_Mouse` AxisValue)) 0.0))) :!label _label_2
      (`|ExecutionSequence`
        (:`then_0`
          (bind (_direction _newtrack_0) (`Timeline|Timeline_1` :!via `Stop` :!label _label_3)
            (:`Update`
              (`SceneComponent.K2_SetRelativeLocation` _springarm (`KismetMathLibrary.MakeVector` (* _relativelocation_x _newtrack_0) (* _relativelocation_y _newtrack_0)) false false))))
        (:`then_1`
          (goto _label_4 :!via `Reset`))
        (:`then_2`
          (`SceneComponent.K2_SetRelativeLocation` _springarm (`KismetMathLibrary.MakeVector` _relativelocation_x_2 (`KismetMathLibrary.FClamp` (+ (* _returnvalue 10.0) _relativelocation_y_2) -1000.0 1000.0) _relativelocation_z) false false)))
      (else
        (`/Engine/EditorBlueprintResources/StandardMacros.DoOnce` false :!label _label_4
          (:`Completed`
            (goto _label_3 :!via `PlayFromStart`)))))))

(event `InputAxis|Move_Front`
  (params (AxisValue :type "Float (single-precision)"))
  ;[0 0.5 1] Character Move
  (goto _label))

(event `InputAxis|Camera_MoveSide_Pad`
  (params (AxisValue :type "Float (single-precision)"))
  ;[0 1 1] Camera Move
  (if (not (`/Game/02_Blueprints/BP_GameInstance.MouseMode` (`self.BP_GameInstance`)))
    (goto _label_2)))

(event `/Game/02_Blueprints/Interfaces/BPI_Character.MoveSide`
  (params (MoveSide :type "Float (single-precision)"))
  ;[0 0.5 1] Character Move
  (bind _returnvalue (select `bool` (`/Game/02_Blueprints/BP_GameInstance.MouseMode` (`self.BP_GameInstance`)) :`false` MoveSide :`true` (stale `InputAxis|Move_Side` AxisValue)))
  (`self.AddMovementInput` (0.0 1.0 0.0) _returnvalue :!label _label_5)
  (if (< (`KismetMathLibrary.Abs` (select `bool` (`/Game/02_Blueprints/BP_GameInstance.MouseMode` (`self.BP_GameInstance`)) :`false` (stale `/Game/02_Blueprints/Interfaces/BPI_Character.MoveFront` MoveFront) :`true` (stale `InputAxis|Move_Front` AxisValue))) (`KismetMathLibrary.Abs` _returnvalue))
    (`/Engine/EditorBlueprintResources/StandardMacros.DoOnce` false :!label _label_6
      (:`Completed`
        (`PaperFlipbookComponent.SetFlipbook` (`self.CharacterFlipbook`) "/Game/05_GA/Assets/MainCharacter/FlipBook/FlipBook_mainChara_WalkSide.FlipBook_mainChara_WalkSide")))
    (else
      (`|ExecutionSequence`
        (:`then_0`
          (goto _label_6 :!via `Reset`))
        (:`then_1`
          _))))
  (if (!= _returnvalue 0.0)
    (`SceneComponent.K2_SetRelativeRotation` (`self.CharacterFlipbook`) (`KismetMathLibrary.MakeRotator` -90.0 (select `bool` (>= _returnvalue 0.0) :`false` 180.0 :`true` 0.0 :!type "Float (single-precision)") 90.0) false false)))

(event `InputAxis|Move_Side`
  (params (AxisValue :type "Float (single-precision)"))
  ;[0 0.5 1] Character Move
  (goto _label_5))

(event `InputAction|Run`
  (params (Key :type "Key Structure"))
  (bind _charactermovement (`self.CharacterMovement`))
  ;[0 0.5 1] Character Move
  (:`Pressed`
    (if (`self.IsWalking?`)
      (set `CharacterMovementComponent.MaxWalkSpeed` 1200.0 _charactermovement)))
  (:`Released`
    (set `CharacterMovementComponent.MaxWalkSpeed` 600.0 _charactermovement)))

(event `InputAxis|Camera_MoveUpDown_Mouse`
  (params (AxisValue :type "Float (single-precision)"))
  (bind _springarm (`self.SpringArm`))
  (bind (_relativelocation_x _relativelocation_y _relativelocation_z) (`KismetMathLibrary.BreakVector` (`SceneComponent.RelativeLocation` _springarm)))
  (bind _mousemode (`/Game/02_Blueprints/BP_GameInstance.MouseMode` (`self.BP_GameInstance`)))
  ;[0 1 1] Camera Move
  (if _mousemode
    (`SceneComponent.K2_SetRelativeLocation` _springarm (`KismetMathLibrary.MakeVector` (`KismetMathLibrary.FClamp` (+ (* (select `bool` _mousemode :`false` (stale `InputAxis|Camera_MoveUpDown_Pad` AxisValue) :`true` AxisValue) 10.0) _relativelocation_x) -500.0 500.0) _relativelocation_y _relativelocation_z) false false :!label _label_7)))

(event `InputAxis|Camera_MoveUpDown_Pad`
  (params (AxisValue :type "Float (single-precision)"))
  ;[0 1 1] Camera Move
  (if (not (`/Game/02_Blueprints/BP_GameInstance.MouseMode` (`self.BP_GameInstance`)))
    (goto _label_7)))

(event `self.FrontCollisionBox.OnComponentBeginOverlap`
  (params (OverlappedComponent :type "PrimitiveComponent Object Reference") (OtherActor :type "Actor Object Reference") (OtherComp :type "PrimitiveComponent Object Reference") (OtherBodyIndex :type Integer) (bFromSweep :type Boolean) (SweepResult :type "HitResult Structure (by ref)"))
  ;[1 1 1] Events Collect
  (set `self.SomethingIn?` true)
  (set `self.ObjectInBox` OtherActor))

(event `self.FrontCollisionBox.OnComponentEndOverlap`
  (params (OverlappedComponent :type "PrimitiveComponent Object Reference") (OtherActor :type "Actor Object Reference") (OtherComp :type "PrimitiveComponent Object Reference") (OtherBodyIndex :type Integer))
  ;[1 1 1] Events Collect
  (set `self.SomethingIn?` false))

(event `InputAction|GetObject`
  (params (Key :type "Key Structure"))
  ;[1 1 1] Events Collect
  (:`Pressed`
    (if (`self.SomethingIn?`) :!label _label_8
      (bind _seedname (message `/Game/02_Blueprints/Interfaces/BPI_Soil.SOIL_GetPlant` (`self.ObjectInBox`)))
      (message `/Game/02_Blueprints/Interfaces/BPI_Inventaire.NewElementInventaire` (`self.Widget_Inventaire`) _seedname))))

(event `/Game/02_Blueprints/Interfaces/BPI_Character.Event_Jump`
  ;[1 1 1] Events Collect
  (goto _label_8))

(event `/Game/02_Blueprints/Interfaces/BPI_Character.Degats`
  (bind _bp_gameinstance (`self.BP_GameInstance`))
  (bind _output_get (set `/Game/02_Blueprints/BP_GameInstance.Character_Life` (- (`/Game/02_Blueprints/BP_GameInstance.Character_Life` _bp_gameinstance) 20) _bp_gameinstance))
  (if (<= _output_get 0)
    (bind _returnvalue (`|CreateWidget` "/Game/02_Blueprints/Widget/Widget_Death.Widget_Death_C"))
    (`UserWidget.AddToViewport` _returnvalue 0)
    (`KismetSystemLibrary.Delay` 3.0)
    (`GameplayStatics.OpenLevel` "Map_MainMenu")
    (set `/Game/02_Blueprints/BP_GameInstance.OnMenuMap` true (`self.BP_GameInstance`))
    (else
      (message `/Game/02_Blueprints/Interfaces/BPI_Character.LessLife` (`self.Widget_Inventaire`)))))

(event `InputAction|Attack`
  (params (Key :type "Key Structure"))
  (bind _arrow1 (`self.Arrow1`))
  (:`Pressed`
    (bind _returnvalue (`|SpawnActorFromClass` "/Game/02_Blueprints/Character/BP_Bullet.BP_Bullet_C" (`SceneComponent.K2_GetComponentToWorld` _arrow1) "AlwaysSpawn" "OverrideRootScale" null null))
    (set `MovementComponent.Velocity` (* (`SceneComponent.GetForwardVector` _arrow1) 400.0) (`/Game/02_Blueprints/Character/BP_Bullet.ProjectileMovement` _returnvalue))))

(fn `UserConstructionScript`)